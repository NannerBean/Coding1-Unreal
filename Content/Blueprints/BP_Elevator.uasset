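; BP_Elevator is an elevator whose platform travels between a Start and an End transform when something overlaps its Box trigger.
; Each overlap flips IsMovingUP, alternately playing and reversing the PlatformMovement timeline, with no filter on the overlapping actor.
; The timeline's Moving track drives a transform lerp that sets the platform's world location and rotation on every update.
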(event OnComponentBeginOverlap(Box)
  (params (OverlappedComponent :type Primitive%20Component%20Object%20Reference) (OtherActor :type Actor%20Object%20Reference) (OtherComp :type Primitive%20Component%20Object%20Reference) (OtherBodyIndex :type Integer) (bFromSweep :type Boolean) (SweepResult :type Hit%20Result%20Structure%20%28by%20ref%29))
  (if (Variables|Default|GetIsMovingUP)
    (Variables|Default|SetIsMovingUP false)
    (bind _moving (Timeline|PlatformMovement Reverse)
      (:Update
        (Transformation|SetWorldLocationAndRotation (Variables|Default|GetPlatform) (.location (Math|Transform|Lerp(Transform) (Transformation|GetWorldTransform (Variables|Default|GetStart)) (Transformation|GetWorldTransform (Variables|Default|GetEnd)) _moving)) (.rotation (Math|Transform|Lerp(Transform) (Transformation|GetWorldTransform (Variables|Default|GetStart)) (Transformation|GetWorldTransform (Variables|Default|GetEnd)) _moving)) false false)))
    (else
      (Variables|Default|SetIsMovingUP true)
      (Timeline|PlatformMovement Play))))

(fn ConstructionScript)