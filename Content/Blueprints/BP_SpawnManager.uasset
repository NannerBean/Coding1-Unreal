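; Spawn manager that runs enemy waves by triggering every BP_EnemySpawner in the level.
; NewEnemyWaveCheck looks for remaining BP_Enemy actors; when none are left, it starts the next wave and spawns a BP_Key at the supplied transform.
; SpawnNewEnemies waits out a short delay, then calls SpawnNewEnemy on each spawner found by class lookup, printing randomly colored debug messages.
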(event Custom|Spawn%20New%20Enemies
  (Development|PrintString "Spawning new enemies in 4 seconds..." true true "(R=1.000000,G=0.052083,B=0.101730,A=1.000000)")
  (Utilities|FlowControl|Delay 4.0)
  (bind _outactors (Actor|GetAllActorsOfClass "/Game/Blueprints/BP_EnemySpawner.BP_EnemySpawner_C"))
  (for (_array_element _array_index) _outactors
    (Default|SpawnNewEnemy _array_element)
    (Development|PrintString (Utilities|String|Append (Utilities|String|ToString(Integer) _array_index) "." (Utilities|GetDisplayName _array_element) " is spawniing...") true true (Utilities|Struct|MakeLinearColor (Math|Random|RandomFloatinRange 0.5 1.0) (Math|Random|RandomFloatinRange 0.5 1.0) (Math|Random|RandomFloatinRange 0.5 1.0) 1.0) 5.0))
  (Development|PrintString "Spawn Complete!" true true "(R=1.000000,G=0.016331,B=0.136021,A=1.000000)"))

(event Custom|New%20Enemy%20Wave%20Check
  (params (Transform :type Transform))
  (bind _outactors (Actor|GetAllActorsOfClass "/Game/Blueprints/BP_Enemy.BP_Enemy_C"))
  (if (> (Utilities|Array|Length _outactors) 0)
    (Development|PrintString "There are still enemies here!")
    (else
      (CallFunction|SpawnNewEnemies)
      (Game|SpawnActorfromClass "/Game/Blueprints/BP_Key.BP_Key_C" Transform "Undefined" "MultiplyWithRoot" 0 0))))

(event EventBeginPlay
  (Development|PrintString "Spawn Manager is Active!" true true "(R=0.238073,G=1.000000,B=0.092520,A=1.000000)")
  (bind _outactors (Actor|GetAllActorsOfClass "/Game/Blueprints/BP_EnemySpawner.BP_EnemySpawner_C"))
  (Development|PrintString (Utilities|String|Append "There are " (Utilities|String|ToString(Integer) (Utilities|Array|Length _outactors)) " spawners in the Level." " There are " "##" " enemies in the level.")))

(fn ConstructionScript)