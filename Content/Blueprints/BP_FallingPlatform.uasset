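; Falling platform that drops some time after the third-person character overlaps it, then returns to its start position.
; An overlap while ready starts a chain of Activate, Falling and Reset events separated by delays, with a material swap marking each state.
; Falling turns on physics simulation; Reset turns it off and a timeline lerps the transform back to the one saved at BeginPlay, then re-arms the platform.
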(event Custom|Activate
  (Rendering|Material|SetMaterial (Variables|Default|GetPlatform) 0 "/Game/Materials/FallingPlatform/MI_PlatformActive.MI_PlatformActive")
  (Variables|Default|SetIsReady false)
  (Development|PrintString "Countdown started...")
  (Utilities|FlowControl|Delay (Variables|PlatformSettings|GetFallDelayDuration))
  (CallFunction|Falling))

(event Custom|Falling
  (Development|PrintString "Falling!" true true "(R=1.000000,G=0.824974,B=0.079861,A=1.000000)")
  (Rendering|Material|SetMaterial (Variables|Default|GetPlatform) 0 "/Game/Materials/FallingPlatform/MI_PlatformFalling.MI_PlatformFalling")
  (Physics|SetSimulatePhysics (Variables|Default|GetPlatform) true) ; Platform is now affected by physics (gravity).
  (Utilities|FlowControl|Delay (Variables|PlatformSettings|GetFallingDuration))
  (CallFunction|Reset))

(event Custom|Reset
  (Development|PrintString "Reseting" true true "(R=1.000000,G=0.795974,B=0.045139,A=1.000000)")
  (Rendering|Material|SetMaterial (Variables|Default|GetPlatform) 0 "/Game/Materials/FallingPlatform/MI_PlatformResetting.MI_PlatformResetting")
  (Physics|SetSimulatePhysics (Variables|Default|GetPlatform) false) ; Platform is now affected by physics (gravity).
  (Variables|Default|SetFallingTransform (Transformation|GetWorldTransform (Variables|Default|GetPlatform)))
  (bind _newtrack_0 (Timeline|GoBackToStartTransform PlayFromStart)
    (:Update
      (Transformation|SetWorldTransform (Variables|Default|GetPlatform) (Math|Transform|Lerp(Transform) (Variables|Default|GetFallingTransform) (Variables|Default|GetStartingTransform) _newtrack_0) false false))
    (:Finished
      (Variables|Default|SetIsReady true)
      (Rendering|Material|SetMaterial (Variables|Default|GetPlatform) 0 "/Game/Materials/FallingPlatform/MI_PlatformReady.MI_PlatformReady"))))

(event EventBeginPlay
  (Variables|Default|SetStartingTransform (Transformation|GetWorldTransform (Variables|Default|GetPlatform))))

(event Collision|EventActorBeginOverlap
  (params (OtherActor :type Actor%20Object%20Reference))
  (Development|PrintString "There's something stadning on me!" true true "(R=1.000000,G=0.887523,B=0.031250,A=1.000000)")
  (Utilities|Casting|CastToBP_ThirdPersonCharacter OtherActor)
  (if (Variables|Default|GetIsReady)
    (CallFunction|Activate)
    (else
      (Development|PrintString "Not Ready  yet!" true true "(R=1.000000,G=0.010417,B=0.142950,A=1.000000)"))))

(fn ConstructionScript)